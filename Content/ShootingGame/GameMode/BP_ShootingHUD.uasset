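; BP_ShootingHUD is the shooting game's HUD Blueprint, relaying the local player's health, ammo and magazine updates to the on-screen widget.
; Three update events each cast the stored HudWidget reference to the HudWidget class and call SetHp, SetAmmo or SetMag with the received values.
; The ammo event also prints a debug string, and widget creation is not handled in these graphs.
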(event EventOnUpdateMyAmmo
  (params (Ammo :type Integer))
  (Development|PrintString "UpdateMyAmmo")
  (bind _ashud_widget (Utilities|Casting|CastToHudWidget (Variables|Default|GetHudWidget)))
  (Default|SetAmmo _ashud_widget Ammo))

(event EventOnUpdateMyMag
  (params (Mag :type Integer))
  (bind _ashud_widget (Utilities|Casting|CastToHudWidget (Variables|Default|GetHudWidget)))
  (Default|SetMag _ashud_widget Mag))

(event EventOnUpdateMyHp
  (params (CurHp :type Float%20%28single-precision%29) (MaxHp :type Float%20%28single-precision%29))
  (bind _ashud_widget (Utilities|Casting|CastToHudWidget (Variables|Default|GetHudWidget)))
  (Default|SetHp _ashud_widget CurHp MaxHp))

(fn ConstructionScript)